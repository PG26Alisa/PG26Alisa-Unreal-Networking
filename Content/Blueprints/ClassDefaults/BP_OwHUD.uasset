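; BP_OwHUD is a HUD Blueprint that shows the WBP_HUD widget for the player's possessed pawn.
; Shortly after BeginPlay, it binds to the owning controller's possessed-pawn-changed delegate and fires the handler for the currently controlled pawn.
; On each pawn change it removes the existing widget, then creates a fresh one and adds it to the viewport if the new pawn is valid.
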(event Custom|OnPossessedPawnChanged_Event
  (params (OldPawn :type Pawn%20Object%20Reference) (NewPawn :type Pawn%20Object%20Reference))
  (bind _playerhud (Variables|Default|GetPlayerHUD)
    (:then
      (Widget|RemovefromParent _playerhud))
    (:else
      _))
  (if (Utilities|IsValid NewPawn)
    (bind _returnvalue (UserInterface|CreateWidget "/Game/UI/WBP_HUD.WBP_HUD_C" (Variables|Default|GetPlayerOwner)))
    (bind _output_get (Variables|Default|SetPlayerHUD _returnvalue))
    (UserInterface|Viewport|AddtoViewport _output_get 0)))

(event EventBeginPlay
  (Utilities|FlowControl|Delay 0.2)
  (bind _playerowner (Variables|Default|GetPlayerOwner)
    (:then
      (EventDispatchers|AssignOnPossessedPawnChanged _playerowner (delegate Custom|OnPossessedPawnChanged_Event))
      (CallFunction|OnPossessedPawnChangedEvent 0 (Pawn|GetControlledPawn _playerowner)))
    (:else)))

(fn ConstructionScript)