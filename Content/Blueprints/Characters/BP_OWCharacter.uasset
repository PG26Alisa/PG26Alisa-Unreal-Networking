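; BP_OWCharacter is a player character Blueprint that binds Enhanced Input actions for movement, shooting, dashing and sprinting.
; Movement follows the actor's forward and right vectors, while the other actions call Shoot, PlayVFX, Dashing, SprintStart and SprintEnd, none of which are defined here.
; HealthComponent updates print old and new health and destroy the actor at zero or below.
; OnVFXPlayed is empty, and an emitter spawn node is left unconnected.
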(event OnHealthUpdated(HealthComponent)
  (params (HealthComponent :type Health%20Component%20Object%20Reference) (OldHealth :type Float%20%28single-precision%29) (NewHealth :type Float%20%28single-precision%29))
  (Development|PrintString (Utilities|String|ToString(Text) (Utilities|Text|FormatText "Old Health {OH}  New Health {NH}" OldHealth NewHealth)) true true "(R=0.000000,G=0.660000,B=1.000000,A=1.000000)" 5.0)
  (if (<= NewHealth 0.0)
    (Actor|DestroyActor)))

(event Input|EnhancedActionEvents|EnhancedInputActionIA_OWDash
  (params (ActionValue :type Boolean) (ElapsedSeconds :type Float%20%28double-precision%29) (TriggeredSeconds :type Float%20%28double-precision%29) (InputAction :type Input%20Action%20Object%20Reference :default "/Game/Inputs/IA_OWDash.IA_OWDash"))
  (Class|OWCharacter|Dashing))

(event Input|EnhancedActionEvents|EnhancedInputActionIA_OWSprint
  (params (ActionValue :type Boolean) (ElapsedSeconds :type Float%20%28double-precision%29) (TriggeredSeconds :type Float%20%28double-precision%29) (InputAction :type Input%20Action%20Object%20Reference :default "/Game/Inputs/IA_OWSprint.IA_OWSprint"))
  (:Triggered
    (Class|OWCharacter|SprintStart))
  (:Completed
    (Class|OWCharacter|SprintEnd)))

(event Input|EnhancedActionEvents|EnhancedInputActionIA_OWShoot
  (params (ActionValue :type Boolean) (ElapsedSeconds :type Float%20%28double-precision%29) (TriggeredSeconds :type Float%20%28double-precision%29) (InputAction :type Input%20Action%20Object%20Reference :default "/Game/Inputs/IA_OWShoot.IA_OWShoot"))
  (Class|OWCharacter|Shoot)
  (Class|OWCharacter|PlayVFX))

(event Input|EnhancedActionEvents|EnhancedInputActionIA_OWMovement
  (params (ActionValue :type Vector%202D%20Structure) (ElapsedSeconds :type Float%20%28double-precision%29) (TriggeredSeconds :type Float%20%28double-precision%29) (InputAction :type Input%20Action%20Object%20Reference :default "/Game/Inputs/IA_OWMovement.IA_OWMovement"))
  (bind (_x _y) (Math|Vector2D|BreakVector2D ActionValue))
  (Pawn|Input|AddMovementInput (Transformation|GetActorForwardVector) _x false)
  (Pawn|Input|AddMovementInput (Transformation|GetActorRightVector) _y false))

(event EventOnVFXPlayed)

(fn ConstructionScript)